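; BP_Controller is the controller that sets up input and the main HUD and relays kill progress to it.
; On BeginPlay it adds the IMC_Game Enhanced Input mapping context, then creates WBP_MainUI and adds it to the viewport.
; It binds to BP_GameMode's kill count update event and forwards current and target kills to the widget, so the UI updates without Tick.
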(event `self.ReceiveBeginPlay`
  (`EnhancedInputSubsystemInterface.AddMappingContext` (subsystem `EnhancedInputLocalPlayerSubsystem`) "/Game/Blueprints/Input/IMC_Game.IMC_Game" 0 (struct))
  ; 위젯 생성및 화면에 출력
  (bind _returnvalue (`|CreateWidget` "/Game/UI/WBP_MainUI.WBP_MainUI_C"))
  (bind _output_get (set `self.MainUI` _returnvalue))
  (`UserWidget.AddToViewport` _output_get 0)
  (bind _asbp_game_mode (cast `/Game/Blueprints/Character/BP_GameMode` (`GameplayStatics.GetGameMode`)))
  (add `/Game/Blueprints/Character/BP_GameMode.OnKillCountUpdate` _asbp_game_mode (delegate `OnKillCountUpdate`)))

(event `OnKillCountUpdate`
  (params (CurrentKills :type Integer) (TargetKills :type Integer))
  (`/Game/UI/WBP_MainUI.OnKillCountUpdated` (`self.MainUI`) CurrentKills TargetKills))

(fn `UserConstructionScript`)