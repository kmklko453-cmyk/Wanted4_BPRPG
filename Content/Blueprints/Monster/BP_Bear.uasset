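; BP_Bear is a bear monster that spots, chases and attacks the player, with hit and death effects.
; A state change updates the AI blackboard and walk speed, and PawnSensing switches Locomotion to Chase on seeing a Player-tagged pawn.
; Damage goes to BPHPController, whose death event disables capsule collision, then after a delay dissolves the mesh and destroys the actor.
; PlayerWeapon overlaps flash the mesh material through a timeline.
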(event `UpdateState`
  (params (NewState :type "/Game/Blueprints/Monster/EBearState Enum" :default "NewEnumerator0"))
  (bind _charactermovement (`self.CharacterMovement`))
  ; 몬스터 상태 변경 이벤트
  (if (`|EnumInequality` (`self.State_BP`) "NewEnumerator3")
    (bind _output_get (set `self.State_BP` NewState))
    (`BlackboardComponent.SetValueAsEnum` (`AIController.Blackboard` (`AIBlueprintHelperLibrary.GetAIController` self)) (`self.StateKey`) _output_get)
    (switch `/Game/Blueprints/Monster/EBearState` (`self.State_BP`)
      (:`NewEnumerator0`
        (set `CharacterMovementComponent.MaxWalkSpeed` 200.0 _charactermovement))
      (:`NewEnumerator1`
        (set `CharacterMovementComponent.MaxWalkSpeed` 500.0 _charactermovement))
      (:`NewEnumerator2`
        (set `CharacterMovementComponent.MaxWalkSpeed` 0.0 _charactermovement :!label _label))
      (:`NewEnumerator3`
        (goto _label)))))

(event `self.ReceiveBeginPlay`
  ;[0.15 0.001228 0.001228 0.5] 죽음 이벤트에 바인딩
  (add `/Game/Blueprints/Components/BP_HPController.OnDeadEvent` (`self.BP_HPController`) (delegate `ReceiveOnDead`)))

(event `ReceiveOnDead`
  (bind _mesh (`self.Mesh`))
  ;[0.15 0.001228 0.001228 0.5] 죽음 이벤트에 바인딩
  (`self.UpdateState` "NewEnumerator3")
  (`PrimitiveComponent.SetCollisionEnabled` (`self.CapsuleComponent`) "NoCollision")
  (`KismetSystemLibrary.Delay` 2.0)
  (bind (_direction _dissolve _hitvalue) (`Timeline|DeathEffect` :!via `PlayFromStart`)
    (:`Update`
      (`MeshComponent.SetScalarParameterValueOnMaterials` _mesh "Dissolve" _dissolve)
      (`MeshComponent.SetScalarParameterValueOnMaterials` _mesh "HitValue" _hitvalue))
    (:`Finished`
      (`self.K2_DestroyActor`))))

(event `self.ReceiveActorBeginOverlap`
  (params (OtherActor :type "Actor Object Reference"))
  ; Overlap발생시 HItEffect
  (if (`self.ActorHasTag` OtherActor "PlayerWeapon")
    (bind (_direction _hitvalue) (`Timeline|HitEffect` :!via `PlayFromStart`)
      (:`Update`
        (`MeshComponent.SetScalarParameterValueOnMaterials` (`self.Mesh`) "HitValue" _hitvalue)))))

(event `self.ReceiveAnyDamage`
  (params (Damage :type "Float (single-precision)") (DamageType :type "DamageType Object Reference") (InstigatedBy :type "Controller Object Reference") (DamageCauser :type "Actor Object Reference"))
  ; 데미지 처리
  (`/Game/Blueprints/Components/BP_HPController.ReceiveDamage` (`self.BP_HPController`) Damage))

(event `self.PawnSensing.OnSeePawn`
  (params (Pawn :type "Pawn Object Reference"))
  ; 시야 감지
  (if (`|EnumEquality` (`self.State_BP`) "NewEnumerator0")
    (if (`self.ActorHasTag` Pawn "Player")
      (`BlackboardComponent.SetValueAsObject` (`AIController.Blackboard` (`AIBlueprintHelperLibrary.GetAIController` self)) (`self.TargetPlayerKey`) Pawn)
      (`self.UpdateState` "NewEnumerator1"))))

(fn `UserConstructionScript`)