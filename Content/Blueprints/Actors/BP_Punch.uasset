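; BP_Punch is a one-shot launcher actor that throws an overlapping Character upward.
; On overlap it sets the mesh material's Alpha parameter to 1, spawns a scaled-up explosion emitter, applies a vertical velocity-change impulse of PunchPower through CharacterMovement, then destroys itself.
; The Alpha highlight also triggers for non-Character actors, which are not launched, and resets when the overlap ends.
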(event `self.ReceiveActorBeginOverlap`
  (params (OtherActor :type "Actor Object Reference"))
  (`MeshComponent.SetScalarParameterValueOnMaterials` (`self.StaticMesh`) "Alpha" 1.0)
  ;[0.15 0 0 0.5] 캐릭터를 위로 올리는 로직
  (bind _ascharacter (cast `Character` OtherActor))
  (`GameplayStatics.SpawnEmitterAtLocation` "/Game/Particles/P_Explosion.P_Explosion" (`self.K2_GetActorLocation`) (struct) (10.0 10.0 10.0))
  (`CharacterMovementComponent.AddImpulse` (`Character.CharacterMovement` _ascharacter) (`KismetMathLibrary.MakeVector` 0.0 0.0 (`self.PunchPower`)) true)
  (`self.K2_DestroyActor`))

(event `self.ReceiveActorEndOverlap`
  (params (OtherActor :type "Actor Object Reference"))
  (`MeshComponent.SetScalarParameterValueOnMaterials` (`self.StaticMesh`) "Alpha" 0.0))

(fn `UserConstructionScript`)